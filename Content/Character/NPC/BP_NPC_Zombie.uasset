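; Zombie NPC that patrols points, hunts the player and plays random-interval growls.
; An enum state drives it: Tick checks distance and an eye-socket line trace, switching patrol to a watching stare that becomes aggro after a delay.
; Aggro chases via AIMoveTo, rechecking only distance before resuming patrol.
; On death it may drop random ammo, then triggers the player's win when no zombies remain.
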(event Custom|GoToNextPoint
  ;[0.15 0.15 0.15 0.5] Patrol
  (if (Utilities|Enum|Equal(Enum) (Variables|StateLogic|GetZombieState) "NewEnumerator0")
    (if (> (Utilities|Array|Length (Variables|Road|GetPatrolPoints)) 0)
      (AI|AIMoveTo (Class|PawnMovementComponent|GetPawnOwner (Variables|Character|GetCharacterMovement)) (Transformation|GetActorLocation (Utilities|Array|Get(acopy) (Variables|Road|GetPatrolPoints) (Variables|Road|GetCurrentPoint))) (Utilities|Array|Get(acopy) (Variables|Road|GetPatrolPoints) (Variables|Road|GetCurrentPoint)) (Variables|Road|GetAcceptanceRadius) true
        (:OnSuccess
          (Utilities|FlowControl|Delay (Variables|/Game/Character/NPC/BP_PatrolPoint.BP_PatrolPoint_C|GetWaitTime (Utilities|Array|Get(acopy) (Variables|Road|GetPatrolPoints) (Variables|Road|GetCurrentPoint))))
          (if (== (- (Utilities|Array|Length (Variables|Road|GetPatrolPoints)) 1) (Variables|Road|GetCurrentPoint))
            (Variables|Road|SetCurrentPoint 0)
            (else
              (Math|Integer|IncrementInt (Variables|Road|GetCurrentPoint)
                (:%20%20
                  _))))
          (CallFunction|GotoNextPoint))))))

(event Custom|StartLookingAtPlayer
  ;[0.15 0.15 0.15 0.5] Look at player
  (Variables|StateLogic|SetZombieState "NewEnumerator1")
  (AI|Navigation|StopMovement (AI|GetAIController self))
  (Utilities|FlowControl|Delay (Variables|StateLogic|GetTimeToLookAtPlayer))
  (if (Utilities|Enum|Equal(Enum) (Variables|StateLogic|GetZombieState) "NewEnumerator1")
    (CallFunction|AgrotoPlayer)))

(event Custom|AgroToPlayer
  ;[0.15 0.15 0.15 0.5] Twitter Behaviour (Agro)
  (Variables|StateLogic|SetZombieState "NewEnumerator2")
  (AI|AIMoveTo self "0, 0, 0" (Game|Player|GetPlayerPawn 0) 5.0 false
    (:then
      (CallFunction|BUEEUEUEUEUERRRRR)
      (Utilities|FlowControl|Delay (Variables|StateLogic|GetDropAgroDuration))
      (if (< (Math|Vector|Distance(Vector) (Transformation|GetActorLocation) (Transformation|GetActorLocation (Game|GetPlayerCharacter 0))) (Variables|Stats|GetVisionDistance))
        (CallFunction|AgrotoPlayer)
        (else
          (CallFunction|StartPatroling))))))

(event Custom|StartPatroling
  ;[0.15 0.15 0.15 0.5] Patrol
  (Variables|StateLogic|SetZombieState "NewEnumerator0")
  (CallFunction|GotoNextPoint))

(event Custom|BUEEUEUEUEUERRRRR
  ;[0.15 0.15 0.15 0.5] On Start
  ;;[0.15 0.15 0.15 0.5] Brrr voice on random for scary vibe
  (Audio|PlaySoundatLocation "/Game/Sounds/Zombie/SC_Zombie_Voice.SC_Zombie_Voice" (Transformation|GetActorLocation) "0, 0, 0" 1.0 1.0 0.0 0 0 0 0))

(event EventBeginPlay
  ;[0.15 0.15 0.15 0.5] On Start
  (Utilities|FlowControl|Sequence
    (:then_0
      ;;[0.15 0.15 0.15 0.5] Set current Health
      (Variables|Stats|SetCurrentHealth (Variables|Stats|GetMaxHealth%20)))
    (:then_1
      ;;[0.15 0.15 0.15 0.5] Set Max Speed
      (Variables|/Script/Engine.CharacterMovementComponent|SetMaxWalkSpeed (Variables|Character|GetCharacterMovement) (Variables|Stats|GetMoveSpeed)))
    (:then_2
      ;;[0.15 0.15 0.15 0.5] Shuffle if needed
      (if (Variables|Road|GetDoRandomRoadOrder)
        (bind _newroad (CallFunction|ShuffleRoad (Variables|Road|GetPatrolPoints)))
        (Variables|Road|SetPatrolPoints _newroad)))
    (:then_3
      ;;[0.15 0.15 0.15 0.5] Go to first point at start
      (if (> (Utilities|Array|Length (Variables|Road|GetPatrolPoints)) 0)
        (CallFunction|GotoNextPoint)))
    (:then_4
      ;;[0.15 0.15 0.15 0.5] Brrr voice on random for scary vibe
      (Utilities|Time|SetTimerbyEvent (delegate Custom|BUEEUEUEUEUERRRRR) (Math|Random|RandomFloatinRange 1e+01 1.2e+02) true))))

(event EventTick
  (params (DeltaSeconds :type Float%20%28single-precision%29))
  (bind _returnvalue (Game|GetPlayerCharacter 0))
  (bind _returnvalue_2 (Transformation|GetActorLocation _returnvalue))
  ;[0.15 0.15 0.15 0.5] See a player logic
  (bind _outhit (Collision|LineTraceByChannel (Transformation|GetSocketLocation (Variables|Character|GetMesh) "LeftEyeSocket") _returnvalue_2 "TraceTypeQuery1" false 0 "None"))
  (switch Utilities|FlowControl|Switch|SwitchonE_ZombieState (Variables|StateLogic|GetZombieState)
    (:NewEnumerator0
      (if (and (< (Math|Vector|Distance(Vector) (Transformation|GetActorLocation) _returnvalue_2) (Variables|Stats|GetVisionDistance)) (== (.HitActor (Collision|BreakHitResult _outhit)) (Game|Player|GetPlayerPawn 0)))
        (CallFunction|StartLookingatPlayer)))
    (:NewEnumerator1
      (if (and (< (Math|Vector|Distance(Vector) (Transformation|GetActorLocation) _returnvalue_2) (Variables|Stats|GetVisionDistance)) (== (.HitActor (Collision|BreakHitResult _outhit)) (Game|Player|GetPlayerPawn 0)))
        (Transformation|SetActorRotation self (Math|Rotator|FindLookatRotation (Transformation|GetActorLocation self) (Transformation|GetActorLocation (Game|Player|GetPlayerPawn 0))))
        (else
          (CallFunction|StartPatroling))))))

(event Game|Damage|EventAnyDamage
  (params (Damage :type Float%20%28single-precision%29) (DamageType :type Damage%20Type%20Object%20Reference) (InstigatedBy :type Controller%20Object%20Reference) (DamageCauser :type Actor%20Object%20Reference))
  ;[0.15 0.15 0.15 0.5] Receive Dmg
  (Development|PrintText "DMG")
  (bind _output_get (Variables|Stats|SetCurrentHealth (- (Variables|Stats|GetCurrentHealth) Damage)))
  (if (<= _output_get 0.0)
    (CallFunction|DropLoot (Variables|Loot|GetLootChance) (Variables|Loot|GetLootAmmo))
    (Actor|DestroyActor)
    (CallFunction|CheckWinCondition)))

(fn ConstructionScript)

(fn ShuffleRoad
  (params (OldRoad :type Array%20of%20BP%20Patrol%20Point%20Object%20References))
  (bind _returnvalue (Utilities|Array|Length OldRoad))
  (bind _returnvalue_2 (- _returnvalue 1))
  (bind _returnvalue_3 (Math|Random|RandomIntegerinRange 0 _returnvalue_2))
  (LocalVariables|SetResultRoad OldRoad)
  (for (_ _array_index) OldRoad
    (if (not (== _array_index _returnvalue_3))
      (Utilities|Array|Swap (LocalVariables|GetResultRoad) _array_index _returnvalue_3)))
  (return (LocalVariables|GetResultRoad)))

(fn DropLoot
  (params (Chance :type Float%20%28double-precision%29) (LootList :type Map%20of%20BP%20Base%20Ammo%20Pickup%20Class%20References%20to%20Objects))
  (bind _lootammo (Variables|Loot|GetLootAmmo))
  (bind _returnvalue (Utilities|Map|Length LootList))
  (bind _returnvalue_2 (- _returnvalue 1))
  (bind _returnvalue_3 (Math|Random|RandomIntegerinRange 0 _returnvalue_2))
  (bind (_key _value) (Utilities|Map|GetKeyValueByIndex _lootammo _returnvalue_3))
  ;[0.15 0.15 0.15 0.5] Chance to drop and check if needed
  (if (> (Utilities|Map|Length LootList) 0)
    (if (>= Chance (Math|Random|RandomFloatinRange 0.0 1e+02))
      ;[0.15 0.15 0.15 0.5] Setup loot
      (bind _returnvalue_4 (Game|SpawnActorfromClass _key (Math|Transform|MakeTransform (.location (Transformation|GetActorTransform)) "0, 0, 0" "1.000000,1.000000,1.000000") "AlwaysSpawn" "MultiplyWithRoot" 0 0))
      (Variables|/Game/Core/Pickup/BP_Base_Ammo_Pickup.BP_Base_Ammo_Pickup_C|SetAmount _returnvalue_4 (Math|Random|RandomIntegerinRange (Variables|/Game/Core/Pickup/BP_LootRule.BP_LootRule_C|GetMinRandomDropChance _value) (Variables|/Game/Core/Pickup/BP_LootRule.BP_LootRule_C|GetMaxRandomDropChance _value)))
      (Variables|/Game/Core/Pickup/BP_Base_Pickup.BP_Base_Pickup_C|SetbCanPickup _returnvalue_4 true)
      (return))))

(fn CheckWinCondition
  (bind _outactors (Actor|GetAllActorsOfClass "BP_NPC_Zombie_C"))
  (if (<= (Utilities|Array|Length _outactors) 0)
    (bind _asbp_player_character (Utilities|Casting|CastToBP_PlayerCharacter (Game|Player|GetPlayerPawn 0)))
    (Default|PlayerWon _asbp_player_character)
    (else
      (Development|PrintText (Utilities|Text|FormatText "Only {count} zombies are present on the level now" (Utilities|Array|Length _outactors))))))